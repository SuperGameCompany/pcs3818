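; Player character for a platformer, with camera-relative movement, jumping and timed power-ups.
; Look input rotates the spring arm with clamped pitch, and horizontal look also yaws the Cube component.
; The PowerUp action and E key each trigger a different state, reverting after a delay.
; SetPowerUpParameters uses the state enum to index a parameter array driving global and player time dilation, jump velocity and a camera post-process material.
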(event EventBeginPlay)

(event Collision|EventActorBeginOverlap
  (params (OtherActor :type Actor%20Object%20Reference)))

(event EventTick
  (params (DeltaSeconds :type Float%20%28single-precision%29)))

(event Input|ActionEvents|InputActionJump
  (params (Key :type Key%20Structure))
  ;[1 0.6932 0] Basic input
  (:Pressed
    (Character|Jump)))

(event Input|ActionEvents|InputActionPowerUp
  (params (Key :type Key%20Structure))
  ;[1 0.6932 0] Basic input
  (:Pressed
    (CallFunction|SetPowerUpParameters "NewEnumerator1")
    (Utilities|FlowControl|Delay 5.0)
    (CallFunction|SetPowerUpParameters "NewEnumerator0")))

(event Input|AxisEvents|InputAxisMoveForward
  (params (AxisValue :type Float%20%28single-precision%29))
  ;[1 0.6932 0] Basic input
  (Pawn|Input|AddMovementInput (Math|Vector|GetForwardVector (Variables|Default|GetCamera)) AxisValue false))

(event Input|AxisEvents|InputAxisMoveRight
  (params (AxisValue :type Float%20%28single-precision%29))
  ;[1 0.6932 0] Basic input
  (Pawn|Input|AddMovementInput (Math|Vector|GetRightVector (Variables|Default|GetCamera)) AxisValue false))

(event Input|AxisEvents|InputAxisVerticalRotate
  (params (AxisValue :type Float%20%28single-precision%29))
  (bind _springarm (Variables|Default|GetSpringArm))
  (bind _relativerotation (Variables|/Script/Engine.SceneComponent|GetRelativeRotation _springarm))
  ;[1 0.6932 0] Basic input
  (Transformation|SetRelativeRotation _springarm (Math|Rotator|MakeRotator (.roll _relativerotation) (Math|Float|Clamp(Float) (+ (.pitch _relativerotation) AxisValue) -3e+01 3e+01) (.yaw _relativerotation)) false false))

(event Input|AxisEvents|InputAxisHorizontalRotate
  (params (AxisValue :type Float%20%28single-precision%29))
  (bind _springarm (Variables|Default|GetSpringArm))
  (bind _cube (Variables|Default|GetCube))
  (bind _relativerotation (Variables|/Script/Engine.SceneComponent|GetRelativeRotation _springarm))
  (bind _relativerotation_2 (Variables|/Script/Engine.SceneComponent|GetRelativeRotation _cube))
  ;[1 0.6932 0] Basic input
  (Transformation|SetRelativeRotation _springarm (Math|Rotator|MakeRotator (.roll _relativerotation) (.pitch _relativerotation) (+ (.yaw _relativerotation) AxisValue)) false false)
  (Transformation|SetRelativeRotation _cube (Math|Rotator|MakeRotator (.roll _relativerotation_2) (.pitch _relativerotation_2) (+ (.yaw _relativerotation_2) AxisValue)) false false))

(event Input|KeyboardEvents|E
  (params (Key :type Key%20Structure))
  ;[1 0.6932 0] Basic input
  (:Pressed
    (CallFunction|SetPowerUpParameters "NewEnumerator2")
    (Utilities|FlowControl|Delay 5.0)
    (CallFunction|SetPowerUpParameters "NewEnumerator0")))

(fn ConstructionScript)

(fn SetPowerUpParameters
  (params (PowerUp :type EPowerUps%20Enum :default "NewEnumerator0"))
  (Variables|Default|SetPowerUpState PowerUp)
  (Utilities|Time|SetGlobalTimeDilation (.GlobalTimeDilation (Utilities|Struct|BreakSPowerUp (Utilities|Array|Get(acopy) (Variables|Default|GetPowerUpParameters) (Math|Conversions|ToInteger(Byte) (Variables|Default|GetPowerUpState))))))
  (Variables|Default|SetCustomTimeDilation self (.UserTimeDilation (Utilities|Struct|BreakSPowerUp (Utilities|Array|Get(acopy) (Variables|Default|GetPowerUpParameters) (Math|Conversions|ToInteger(Byte) (Variables|Default|GetPowerUpState))))))
  (Variables|/Script/Engine.CharacterMovementComponent|SetJumpZVelocity (Variables|Character|GetCharacterMovement) (.JumpVelocity (Utilities|Struct|BreakSPowerUp (Utilities|Array|Get(acopy) (Variables|Default|GetPowerUpParameters) (Math|Conversions|ToInteger(Byte) (Variables|Default|GetPowerUpState))))))
  (Variables|/Script/Engine.CameraComponent|SetPostProcessSettings (Variables|Default|GetCamera) (Utilities|Struct|MakePostProcessSettings (Utilities|Struct|MakeWeightedBlendables (Utilities|Array|MakeArray (.PostProcessingMaterial (Utilities|Struct|BreakSPowerUp (Utilities|Array|Get(acopy) (Variables|Default|GetPowerUpParameters) (Math|Conversions|ToInteger(Byte) (Variables|Default|GetPowerUpState)))))))))
  (return))