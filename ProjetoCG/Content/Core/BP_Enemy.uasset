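; BP_Enemy is an enemy Blueprint that feeds player targeting and animation timing to its AI Blackboard.
; Every Tick it writes the first player character's mesh location to TargetLocation and the character itself to Target.
; It also sets AttackTimer to the full length of the animation asset on its mesh's single-node anim instance, whichever animation that is.
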(event EventTick
  (params (DeltaSeconds :type Float%20%28single-precision%29))
  (bind _self self)
  (bind _returnvalue (AI|GetBlackboard _self))
  (AI|Components|Blackboard|SetValueasVector _returnvalue (Utilities|Name|MakeLiteralName "TargetLocation") (Transformation|GetWorldLocation (Variables|/Script/Engine.Character|GetMesh (Game|GetPlayerCharacter 0))))
  (AI|Components|Blackboard|SetValueasObject _returnvalue (Utilities|Name|MakeLiteralName "Target") (Game|GetPlayerCharacter 0))
  (bind _returnvalue_2 (Animation|GetPlayLength (.AsAnim%20Sequence%20Base (Utilities|Casting|CastToAnimSequenceBase (Class|AnimSingleNodeInstance|GetAnimationAsset (.AsAnim%20Single%20Node%20Instance (Utilities|Casting|CastToAnimSingleNodeInstance (Components|SkeletalMesh|GetAnimInstance (Variables|Character|GetMesh)))))))))
  (AI|Components|Blackboard|SetValueasFloat _returnvalue (Utilities|Name|MakeLiteralName "AttackTimer") _returnvalue_2))

(fn ConstructionScript)